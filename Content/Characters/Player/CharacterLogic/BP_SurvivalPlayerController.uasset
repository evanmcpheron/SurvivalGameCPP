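; Player controller for the survival game that creates the main UI layout for the local player and pushes its default HUD.
; The inventory input calls an empty OnClientInventory, while a ClientInventory event toggles input mode and cursor, pushing the inventory screen on open.
; Slot update and reset events forward to client events that look up a widget, but the lookup and follow-up logic are unimplemented stubs.
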(event Custom|ClientInventory
  ;[0 0.1469 1] Show/Hide inventory
  (Utilities|FlowControl|Delay 0.1)
  (if (Variables|Default|GetIs%20Inventory%20Visible)
    (Input|SetInputModeGameOnly self false)
    (Variables|Default|SetIs%20Inventory%20Visible false)
    (Variables|Default|SetbShowMouseCursor false)
    (else
      (bind _aswb_main_uilayout (Utilities|Casting|CastToWB_MainUILayout (Variables|Default|GetMainUILayoutRef)))
      (Default|PushGameInventory _aswb_main_uilayout)
      (Input|SetInputModeUIOnly self 0 "DoNotLock" false)
      (Variables|Default|SetIs%20Inventory%20Visible true)
      (Variables|Default|SetbShowMouseCursor true))))

(event Custom|OnClientUpdateSlot
  (params (Container :type UContainerType%20Enum :default "Inventory") (Index :type Integer) (ItemInfo :type Item%20Info%20Object%20Reference))
  ;[0 0.1469 1] Update Item Slot
  (bind _widget (CallFunction|GetInventoryWidget Container Index))
  (Utilities|IsValid _widget))

(event Custom|OnClientReset
  (params (Container :type UContainerType%20Enum :default "Inventory") (Index :type Integer))
  ;[0 0.1469 1] Reset Item Slot
  (bind _widget (CallFunction|GetInventoryWidget Container Index))
  (Utilities|IsValid _widget))

(event Input|EnhancedActionEvents|EnhancedInputActionIA_Inventory
  (params (ActionValue :type Boolean) (ElapsedSeconds :type Float%20%28double-precision%29) (TriggeredSeconds :type Float%20%28double-precision%29) (InputAction :type Input%20Action%20Object%20Reference :default "/Game/Blueprints/Inputs/Actions/IA_Inventory.IA_Inventory"))
  ;[0 0.1469 1] Show/Hide inventory
  (:Started
    (CallFunction|OnClientInventory)))

(event EventBeginPlay
  (Networking|SwitchHasAuthority
    (:Authority
      (if (Pawn|IsLocalPlayerController)
        (bind _returnvalue (Game|ConstructObjectfromClass self "/Game/UI/Widgets/Widgets/WB_MainUILayout.WB_MainUILayout_C" :!label _label))
        (UserInterface|Viewport|AddtoViewport _returnvalue 0)
        (Default|PushDefaultHUD _returnvalue)))
    (:Remote
      (goto _label))))

(event EventResetItemSlot
  (params (Container :type UContainerType%20Enum :default "Inventory") (Index :type Integer))
  ;[0 0.1469 1] Reset Item Slot
  (CallFunction|OnClientReset Container Index))

(event EventUpdateItemSlots
  (params (Container :type UContainerType%20Enum :default "Inventory") (Index :type Integer) (ItemInfo :type Item%20Info%20Object%20Reference))
  ;[0 0.1469 1] Update Item Slot
  (CallFunction|OnClientUpdateSlot Container Index ItemInfo))

(fn ConstructionScript)

(fn OnClientInventory)

(fn GetInventoryWidget
  (params (Container :type UContainerType%20Enum :default "Inventory") (SlowIndex :type Integer))
  (return 0))